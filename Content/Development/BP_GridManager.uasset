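; Grid manager actor that builds a point grid in construction and provides spatial queries for picking locations, similar to a simple EQS.
; Tick ages every point and resets those within range and line of sight of any BP_EnemyCharacter, tracking how long each went unseen.
; Functions filter points by visibility or distance, rate them by distance from actors, and select by score or longest unseen time.
; Debug points shade green to red with age.
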(event Custom|ShowGrid
  (CallFunction|DebugShowGrid 5.0))

(event EventBeginPlay
  (bind _outactors (Actor|GetAllActorsOfClass "/Game/Development/BP_EnemyCharacter.BP_EnemyCharacter_C"))
  (Variables|Default|SetEnemies _outactors)
  (Utilities|FlowControl|Sequence
    (:then_0
      (for _array_element (Variables|Tech|GetGrid)
        (Utilities|Map|Add (Variables|Tech|GetGrid_WithTime) _array_element 1e+01)))
    (:then_1
      (Utilities|FlowControl|Delay 0.2)
      (Actor|Tick|SetActorTickEnabled true))))

(event EventTick
  (params (DeltaSeconds :type Float%20%28single-precision%29))
  (bind _returnvalue (Math|Float|MakeLiteralFloat 5.0))
  (CallFunction|UpTime DeltaSeconds)
  (CallFunction|CleanTime 5e+02)
  (bind _keys (Utilities|Map|Keys (Variables|Tech|GetGrid_WithTime)))
  (for _array_element _keys
    (Rendering|Debug|DrawDebugPoint _array_element 15.0 (Math|Color|Lerp(LinearColor) "(R=0.000000,G=1.000000,B=0.022145,A=1.000000)" "(R=1.000000,G=0.008304,B=0.000000,A=1.000000)" (/ (Math|Float|Clamp(Float) (.Value (Utilities|Map|Find (Variables|Tech|GetGrid_WithTime) _array_element)) 0.0 _returnvalue) _returnvalue)) (+ DeltaSeconds 0.001))))

(fn ConstructionScript
  (CallFunction|GenerateGrid)
  (CallFunction|DebugShowGrid 0.2))

(fn GenerateGrid
  (bind _pointscount (Variables|Settings|GetPointsCount))
  (bind _distance (Variables|Settings|GetDistance))
  (Utilities|Array|Clear (Variables|Tech|GetGrid))
  (for _index (range 1 (.x _pointscount))
    (LocalVariables|Set-X _index)
    (for _index_2 (range 1 (.y _pointscount))
      (LocalVariables|Set-Y _index_2)
      (Utilities|Array|Add (Variables|Tech|GetGrid) (+ (Variables|Settings|GetStartPoint) (Math|Vector|MakeVector (* _distance (LocalVariables|Get-Y)) (* _distance (LocalVariables|Get-X)) 0.0))))))

(fn DebugShowGrid
  (params (Duration :type Float%20%28single-precision%29))
  (for _array_element (Variables|Tech|GetGrid)
    (Rendering|Debug|DrawDebugSphere _array_element 25.0 12 "(R=0.000000,G=0.104230,B=1.000000,A=1.000000)" Duration 2.0)))

(fn GetGridData
  (return (Variables|Tech|GetGrid)))

(fn VisibilityFilter
  (params (InputGrid :type Array%20of%20Vectors) (TestActor :type Actor%20Object%20Reference))
  (LocalVariables|Set-TestingActorLocation (Transformation|GetActorLocation TestActor))
  (for _array_element InputGrid
    (LocalVariables|Set-CurrentPoint _array_element)
    (bind _returnvalue (Collision|LineTraceForObjects (LocalVariables|Get-TestingActorLocation) (LocalVariables|Get-CurrentPoint) (Utilities|Array|MakeArray "ObjectTypeQuery1" "ObjectTypeQuery2") false (Utilities|Array|MakeArray TestActor) "None"))
    (if (not _returnvalue)
      (Utilities|Array|Add (LocalVariables|Get-NewData) (LocalVariables|Get-CurrentPoint))))
  (return (LocalVariables|Get-NewData)))

(fn FurtherfromActorsRate
  (params (InputGrid :type Array%20of%20Vectors) (TestActors :type Array%20of%20Actor%20Object%20References))
  (Utilities|FlowControl|Sequence
    (:then_0
      (for _array_element TestActors
        (Utilities|Array|Add (LocalVariables|Get-TestActorsLocations) (Transformation|GetActorLocation _array_element))))
    (:then_1
      (for _array_element_2 InputGrid
        (LocalVariables|Set-TestLocation _array_element_2)
        (Utilities|FlowControl|Sequence
          (:then_0
            (goto _label Reset))
          (:then_1
            (for _array_element_3 (LocalVariables|Get-TestActorsLocations)
              (LocalVariables|Set-CurrentDistance (Math|Vector|Distance(Vector) _array_element_3 (LocalVariables|Get-TestLocation)))
              (Utilities|FlowControl|Sequence
                (:then_0
                  (Utilities|FlowControl|DoOnce false :!label _label
                    (:Completed
                      (LocalVariables|Set-TestMinDistance (LocalVariables|Get-CurrentDistance)))))
                (:then_1
                  (if (< (LocalVariables|Get-CurrentDistance) (LocalVariables|Get-TestMinDistance))
                    (LocalVariables|Set-TestMinDistance (LocalVariables|Get-CurrentDistance))))
                (:then_2
                  (Utilities|FlowControl|DoOnce false
                    (:Completed
                      (bind _output_get (LocalVariables|Set-GlobalMax (LocalVariables|Get-CurrentDistance)))
                      (LocalVariables|Set-GlobalMin _output_get))))
                (:then_3
                  (if (> (LocalVariables|Get-CurrentDistance) (LocalVariables|Get-GlobalMax))
                    (LocalVariables|Set-GlobalMax (LocalVariables|Get-CurrentDistance))))
                (:then_4
                  (if (> (LocalVariables|Get-CurrentDistance) (LocalVariables|Get-GlobalMax))
                    (LocalVariables|Set-GlobalMax (LocalVariables|Get-CurrentDistance))))))
            (Utilities|Map|Add (LocalVariables|Get-Rated) (LocalVariables|Get-TestLocation) (LocalVariables|Get-TestMinDistance))))))
    (:then_2
      (bind _keys (Utilities|Map|Keys (LocalVariables|Get-Rated)))
      (for _array_element_4 _keys
        (Utilities|Map|Add (LocalVariables|Get-Rated) _array_element_4 (/ (- (.Value (Utilities|Map|Find (LocalVariables|Get-Rated) _array_element_4)) (LocalVariables|Get-GlobalMin)) (- (LocalVariables|Get-GlobalMax) (LocalVariables|Get-GlobalMin))))))
    (:then_3
      (return (LocalVariables|Get-Rated)))))

(fn SelectGridPoint
  (params (InputGrid :type Map%20of%20Vectors%20to%20Reals) (SelectMin :type Boolean))
  (LocalVariables|Set-ValueMultiplier (Math|Float|SelectFloat -1.0 1.0 SelectMin))
  (Utilities|FlowControl|Sequence
    (:then_0
      (bind _keys (Utilities|Map|Keys InputGrid))
      (for _array_element _keys
        (LocalVariables|Set-TestingKey _array_element)
        (LocalVariables|Set-TestingValue (* (.Value (Utilities|Map|Find InputGrid (LocalVariables|Get-TestingKey))) (LocalVariables|Get-ValueMultiplier)))
        (Utilities|FlowControl|Sequence
          (:then_0
            (Utilities|FlowControl|DoOnce false
              (:Completed
                (LocalVariables|Set-MaxValue (LocalVariables|Get-TestingValue))
                (LocalVariables|Set-SelectedKey (LocalVariables|Get-TestingKey)))))
          (:then_1
            (if (> (LocalVariables|Get-TestingValue) (LocalVariables|Get-MaxValue))
              (LocalVariables|Set-MaxValue (LocalVariables|Get-TestingValue))
              (LocalVariables|Set-SelectedKey (LocalVariables|Get-TestingKey)))))))
    (:then_1
      (return (LocalVariables|Get-SelectedKey)))))

(fn UpTime
  (params (Time :type Float%20%28double-precision%29))
  (bind _keys (Utilities|Map|Keys (Variables|Tech|GetGrid_WithTime)))
  (for _array_element _keys
    (Utilities|Map|Add (Variables|Tech|GetGrid_WithTime) _array_element (+ (.Value (Utilities|Map|Find (Variables|Tech|GetGrid_WithTime) _array_element)) Time))))

(fn CleanTime
  (params (CleanDistance :type Float%20%28double-precision%29))
  (bind _keys (Utilities|Map|Keys (Variables|Tech|GetGrid_WithTime)))
  (for _array_element _keys
    (for _array_element_2 (Variables|Default|GetEnemies)
      (if (<= (Math|Vector|Distance(Vector) (Transformation|GetActorLocation _array_element_2) _array_element) CleanDistance)
        (bind _returnvalue (Collision|LineTraceForObjects _array_element (Transformation|GetActorLocation _array_element_2) (Utilities|Array|MakeArray "ObjectTypeQuery1" "ObjectTypeQuery2") false (Utilities|Array|MakeArray _array_element_2) "None"))
        (if (not _returnvalue)
          (Utilities|Map|Add (Variables|Tech|GetGrid_WithTime) _array_element 0.0))))))

(fn DistanceFilter
  (params (InputGrid :type Array%20of%20Vectors) (Location :type Vector) (CutDistance :type Float%20%28double-precision%29))
  (for _array_element InputGrid
    (if (<= (Math|Vector|Distance(Vector) _array_element Location) CutDistance)
      (Utilities|Array|Add (LocalVariables|Get-NewData) _array_element)))
  (return (LocalVariables|Get-NewData)))

(fn SelectbyTime
  (params (InputGrid :type Array%20of%20Vectors))
  (for _array_element InputGrid
    (if (>= (.Value (Utilities|Map|Find (Variables|Tech|GetGrid_WithTime) _array_element)) (LocalVariables|Get-MaxTime))
      (LocalVariables|Set-MaxTime (.Value (Utilities|Map|Find (Variables|Tech|GetGrid_WithTime) _array_element)))
      (LocalVariables|Set-NewPoint _array_element)))
  (return (LocalVariables|Get-NewPoint)))
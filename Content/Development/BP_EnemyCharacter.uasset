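; BP_EnemyCharacter is an enemy that picks its movement goals from a grid manager, with a randomized walk speed set at spawn.
; Each Tick, it filters grid data by visibility from itself and by distance, selects a point by time and moves there.
; An unconnected alternative loop would move it away from line-of-sight fellow enemies, found by GetVisibleFriends traces, using a furthest-from-actors grid rating.
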(event EventTick
  (params (DeltaSeconds :type Float%20%28single-precision%29))
  (bind _gridmanager (CallFunction|GetGridManager))
  (bind _self self)
  (bind _grid (Default|GetGridData _gridmanager))
  (bind _grid_2 (Default|VisibilityFilter _gridmanager _grid _self))
  (bind _grid_3 (Default|DistanceFilter _gridmanager _grid_2 (Transformation|GetActorLocation _self) (Variables|Default|GetCutDistance)))
  (bind _point (Default|SelectbyTime _gridmanager _grid_3))
  (AI|Navigation|SimpleMovetoLocation (Pawn|GetController) _point))

(event EventBeginPlay
  (Variables|/Script/Engine.CharacterMovementComponent|SetMaxWalkSpeed (Variables|Character|GetCharacterMovement) (Math|Random|RandomFloatinRange 3e+02 4e+02)))

(fn ConstructionScript)

(fn GetVisibleFriends
  (LocalVariables|Set-MyLocation (Transformation|GetActorLocation self))
  (Utilities|FlowControl|Sequence
    (:then_0
      (for _array_element (Variables|Default|GetFriends)
        (bind _returnvalue (Collision|LineTraceForObjects (Transformation|GetActorLocation _array_element) (LocalVariables|Get-MyLocation) (Utilities|Array|MakeArray "ObjectTypeQuery1" "ObjectTypeQuery2") false (Utilities|Array|MakeArray _array_element) "None"))
        (if (not _returnvalue)
          (Utilities|Array|Add (LocalVariables|Get-VisibleFriends) _array_element))))
    (:then_1
      (return (LocalVariables|Get-VisibleFriends)))))